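; Cube actor for Stage 3 that slides back and forth between its starting position and a point a short distance along its right vector.
; On BeginPlay it stores both endpoints, and a Timeline drives a lerp between them to set the actor's location without sweeping.
; The Timeline's Finished output feeds back into a FlipFlop that alternates Play and Reverse, so the motion repeats without using Tick.
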(event `self.ReceiveBeginPlay`
  (bind _output_get (set `self.StartLocation` (`self.K2_GetActorLocation`)))
  (set `self.TargetLocation` (+ _output_get (* (`self.GetActorRightVector`) 20.0)))
  (`/Engine/EditorBlueprintResources/StandardMacros.FlipFlop` :!label _label
    (:`A`
      (bind (_direction _output) (`Timeline|Timeline` :!label _label_2)
        (:`Update`
          (`self.K2_SetActorLocation` (`KismetMathLibrary.VLerp` (`self.StartLocation`) (`self.TargetLocation`) _output)))
        (:`Finished`
          (goto _label))))
    (:`B`
      (goto _label_2 :!via `Reverse`))))

(fn `UserConstructionScript`)