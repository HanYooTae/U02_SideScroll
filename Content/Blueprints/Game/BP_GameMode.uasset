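; Stage game mode that decides between stage clear and game over.
; BeginPlay looks up the "Boss"-tagged BP_Mutant, creates hidden clear, pause and game-over widgets, and derives the stage number from the level name.
; Tick polls the boss: its death saves progress in BP_GameInstance, kills other characters once and shows the clear screen after a delay; otherwise player death shows game over.
; KillAllMutant is a cheat that kills every mutant.
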(event `KillAllMutant`
  ;[1 0.269 0.8665] 치트키
  (bind _outactors (`GameplayStatics.GetAllActorsOfClass` "/Game/Blueprints/Characters/BP_Mutant.BP_Mutant_C"))
  (for _array_element _outactors
    (`GameplayStatics.ApplyDamage` _array_element 9999.0)))

(event `self.ReceiveBeginPlay`
  (bind _returnvalue (`GameplayStatics.GetPlayerController` 0))
  ;[1 1 1] Clear Widget 생성 및 숨김
  (bind _outactors (`GameplayStatics.GetAllActorsOfClass` "/Game/Blueprints/Characters/BP_Mutant.BP_Mutant_C"))
  (for _array_element _outactors
    (for _array_element_2 (`Actor.Tags` _array_element)
      (if (== _array_element_2 "Boss")
        (set `self.Boss` _array_element)))
    (bind _returnvalue_2 (`|CreateWidget` "/Game/Widgets/WB_Clear.WB_Clear_C" (`GameplayStatics.GetPlayerController` 0) :!label _label))
    (bind _output_get (set `self.ClearWidget` _returnvalue_2))
    (`UserWidget.AddToViewport` _output_get 0)
    (`Widget.SetVisibility` (`self.ClearWidget`) "Hidden")
    ;[1 1 1] Pause Widget 생성 및 숨김
    (bind _returnvalue_3 (`|CreateWidget` "/Game/Widgets/WB_Pause.WB_Pause_C" (`GameplayStatics.GetPlayerController` 0)))
    (bind _output_get_2 (set `self.PauseWidget` _returnvalue_3))
    (`UserWidget.AddToViewport` _output_get_2 0)
    (`Widget.SetVisibility` (`self.PauseWidget`) "Hidden")
    ;[1 1 1] GameOver Widget 생성 및 숨김
    (bind _returnvalue_4 (`|CreateWidget` "/Game/Widgets/WB_GameOver.WB_GameOver_C" (`GameplayStatics.GetPlayerController` 0)))
    (bind _output_get_3 (set `self.GameOverWidget` _returnvalue_4))
    (`UserWidget.AddToViewport` _output_get_3 0)
    (`Widget.SetVisibility` (`self.GameOverWidget`) "Hidden")
    ;[1 1 1] 맵이 로드되면 입력을 게임전용으로
    (set `PlayerController.bShowMouseCursor` false _returnvalue)
    (`WidgetBlueprintLibrary.SetInputMode_GameOnly` _returnvalue)
    ;[1 1 1] 현재 플레이 중인 스테이지 번호 저장
    (bind _returnvalue_5 (`GameplayStatics.GetCurrentLevelName` true))
    (bind _asbp_game_instance (cast `/Game/Blueprints/Game/BP_GameInstance` (`GameplayStatics.GetGameInstance`)))
    (set `/Game/Blueprints/Game/BP_GameInstance.CurrentStage` (`KismetStringLibrary.Conv_StringToInt` (`KismetStringLibrary.Replace` _returnvalue_5 "Stage")) _asbp_game_instance))
  (goto _label))

(event `self.ReceiveTick`
  (params (DeltaSeconds :type "Float (single-precision)"))
  (bind _returnvalue (`GameplayStatics.GetPlayerController` 0))
  (bind _returnvalue_2 (`GameplayStatics.GetPlayerController` 0))
  (bind _clearwidget (`self.ClearWidget`))
  ;[1 1 1] 스테이지 클리어 조건(보스 사망)
  (bind _boss (`self.Boss`)
    (:`then`
      (if (`|EnumEquality` (`/Game/Blueprints/Characters/BP_Mutant.State` _boss) "NewEnumerator3")
        ;[1 1 1] 클리어 스테이지 번호 저장(단, 이미 클리어했던 스테이지는 제외)
        (bind _asbp_game_instance (cast `/Game/Blueprints/Game/BP_GameInstance` (`GameplayStatics.GetGameInstance`)))
        (bind _currentstage (`/Game/Blueprints/Game/BP_GameInstance.CurrentStage` _asbp_game_instance))
        (if (> _currentstage (`/Game/Blueprints/Game/BP_GameInstance.ClearStage` _asbp_game_instance))
          (set `/Game/Blueprints/Game/BP_GameInstance.ClearStage` _currentstage _asbp_game_instance))
        ;[1 1 1] 클리어 스테이지 번호 저장
        (bind _asbp_game_instance_2 (cast `/Game/Blueprints/Game/BP_GameInstance` (`GameplayStatics.GetGameInstance`)))
        (`/Game/Blueprints/Game/BP_GameInstance.Save` _asbp_game_instance_2)
        ;[1 1 1] 생존한 적 올킬
        (`/Engine/EditorBlueprintResources/StandardMacros.DoOnce` false ; tick을 사용하여 enemy한테 데미지가 계속 들어가는 문제 해결
          (:`Completed`
            (bind _outactors (`GameplayStatics.GetAllActorsOfClass` "/Script/Engine.Character"))
            (for _array_element _outactors
              (cast `/Game/Blueprints/Characters/BP_Player` _array_element
                (:`CastFailed`
                  (`GameplayStatics.ApplyDamage` _array_element 9999.0))))
            ;[1 1 1] Clear Widget 표시
            (`KismetSystemLibrary.Delay` 5.0)
            (`Widget.SetVisibility` _clearwidget "Visible")
            (`UserWidget.PlayAnimation` _clearwidget (`/Game/Widgets/WB_Clear.Expand` _clearwidget) 0.0 1 "Forward" 1.0 false)
            (set `PlayerController.bShowMouseCursor` true _returnvalue)
            (`WidgetBlueprintLibrary.SetInputMode_GameAndUIEx` _returnvalue null)))
        (else
          (bind _asbp_player (cast `/Game/Blueprints/Characters/BP_Player` (`GameplayStatics.GetPlayerCharacter` 0)))
          (if (`/Game/Blueprints/Characters/BP_Player.isDead` _asbp_player)
            (`KismetSystemLibrary.Delay` 3.0)
            (`Widget.SetVisibility` (`self.GameOverWidget`) "Visible")
            (set `PlayerController.bShowMouseCursor` true _returnvalue_2)
            (`WidgetBlueprintLibrary.SetInputMode_UIOnlyEx` _returnvalue_2 null)))))
    (:`else`)))

(fn `UserConstructionScript`)