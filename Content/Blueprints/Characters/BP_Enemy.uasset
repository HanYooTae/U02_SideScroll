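; Sword-wielding enemy character that chases and attacks the player, measuring distance and direction along the Y axis only.
; Tick runs a state machine (Idle, Approach, Attack, Dead), while montage-driven events like EndAttack and Hitted choose the next action.
; Toggled sword collision applies damage to the player.
; Taking damage triggers knockback, material flash and damage text, with CurrentHP's RepNotify updating a spawned HP-bar actor until death.
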(event `self.ReceiveBeginPlay`
  ;[1 1 1] BeginPlay : 다이나믹 머티리얼 생성 및 무기충돌체 끄기 등
  (bind _returnvalue (`KismetMaterialLibrary.CreateDynamicMaterialInstance` "/Game/Mixamo/Enemy/Ch25_body1_Inst.Ch25_body1_Inst"))
  (bind _output_get (set `self.BodyMaterialDynamic` _returnvalue)) ; Material에 연결안하면 NULL
  (`PrimitiveComponent.SetMaterial` (`self.Mesh`) 1 _output_get) ; 값을 갖고있는 앞의 변수에서 값을 불러옴
  (bind _returnvalue_2 (`KismetMaterialLibrary.CreateDynamicMaterialInstance` "/Game/Mixamo/Enemy/Ch25_Body_Inst.Ch25_Body_Inst"))
  (bind _output_get_2 (set `self.HeadMaterialDynamic` _returnvalue_2))
  (`PrimitiveComponent.SetMaterial` (`self.Mesh`) 0 _output_get_2)
  (`PrimitiveComponent.SetCollisionEnabled` (`self.SwordCollision`) "NoCollision")
  ;[1 1 1] HP 위젯 액터 생성
  (bind _returnvalue_3 (`|SpawnActorFromClass` "/Game/Blueprints/etc/BP_EnemyHP.BP_EnemyHP_C" (`KismetMathLibrary.MakeTransform` (`SceneComponent.K2_GetComponentLocation` (`self.HPWidgetSocket`))) "Undefined" "OverrideRootScale" null null))
  (set `self.EnemyHP` _returnvalue_3)
  (set `self.CurrentHP` (`self.MaxHP`)))

(event `DamageEffect`
  ;[1 1 1] 데미지를 입었을 때
  (`self.PlayDamageText`)
  (`MaterialInstanceDynamic.SetVectorParameterValue` (`self.BodyMaterialDynamic`) "HitColor" (struct :`R` 1.0 :`A` 1.0))
  (`MaterialInstanceDynamic.SetVectorParameterValue` (`self.HeadMaterialDynamic`) "HitColor" (struct :`R` 1.0 :`A` 1.0))
  (`KismetSystemLibrary.Delay` 0.1)
  (`MaterialInstanceDynamic.SetVectorParameterValue` (`self.BodyMaterialDynamic`) "HitColor" (struct :`A` 1.0))
  (`MaterialInstanceDynamic.SetVectorParameterValue` (`self.HeadMaterialDynamic`) "HitColor" (struct :`A` 1.0)))

(event `self.ReceiveAnyDamage`
  (params (Damage :type "Float (single-precision)") (DamageType :type "DamageType Object Reference") (InstigatedBy :type "Controller Object Reference") (DamageCauser :type "Actor Object Reference"))
  ;[1 1 1] 데미지를 입었을 때
  (set `self.Damage` Damage)
  (if (`|EnumInequality` (`self.State`) "NewEnumerator3")
    (set `self.isAttacking` false)
    (`PrimitiveComponent.SetCollisionEnabled` (`self.SwordCollision`) "NoCollision")
    (`GameplayStatics.PlaySoundAtLocation` "/Game/Sounds/Hit.Hit" (`self.K2_GetActorLocation`) (struct) 1.0 1.0 0.0 "/Game/Sounds/SA_Hit.SA_Hit" null null)
    (`self.DamageEffect`)
    (bind _output_get (set `self.CurrentHP` (- (`self.CurrentHP`) (`self.Damage`))))
    (if (<= _output_get 0.0)
      (`self.K2_DestroyActor` (`self.EnemyHP`))
      (`self.PlayAnimMontage` "/Game/Mixamo/Enemy/Animations/Dying_Backwards_Montage.Dying_Backwards_Montage" 1.0 "Start")
      (set `self.State` "NewEnumerator3")
      (set `PrimitiveComponent.bGenerateOverlapEvents` false (`self.CapsuleComponent`))
      (else
        (`self.LaunchCharacter` (* (* (`self.DirectionToPlayer`) -1.0) 500.0))
        (`self.PlayAnimMontage` "/Game/Mixamo/Enemy/Animations/Great_Sword_Impact_Montage.Great_Sword_Impact_Montage")
        (set `self.State` "NewEnumerator5")))))

(event `Hitted`
  ;[1 1 1] 데미지를 입었을 때
  (`self.NextState`))

(event `NextState`
  ;[1 1 1] 노티파이 호출용 :  이후에 공격을 할지 추격을 할지
  (if (`self.IsActorTickEnabled`)
    (if (not (`self.IsPlayerDead`))
      (set `self.isAttacking` false)
      (if (> (`self.DistanceToPlayer`) 160.0)
        (set `self.State` "NewEnumerator1")
        (else
          (`self.K2_SetActorRotation` (`KismetMathLibrary.Conv_VectorToRotator` (`self.DirectionToPlayer`)))
          (`self.PlayAnimMontage` "/Game/Mixamo/Enemy/Animations/Great_Sword_Slash_Montage.Great_Sword_Slash_Montage" (`self.AttackSpeed`))
          (set `self.isAttacking` true) ; 공격 몽타주 이후에 공격 상태 true
        )))))

(event `EndAttack`
  ;[1 1 1] EndAttack : 공격종료 및 재공격
  (`self.NextState`))

(event `self.ReceiveTick`
  (params (DeltaSeconds :type "Float (single-precision)"))
  (bind (_returnvalue_x _returnvalue_y) (`KismetMathLibrary.BreakVector` (- (`self.K2_GetActorLocation` (`GameplayStatics.GetPlayerCharacter` 0)) (`self.K2_GetActorLocation`))))
  (bind _returnvalue (`KismetMathLibrary.MakeVector` 0.0 _returnvalue_y))
  ;[1 1 1] 상태 변경
  (bind _enemyhp (`self.EnemyHP`)
    (:`then`
      (`/Game/Blueprints/etc/BP_EnemyHP.Update Location` _enemyhp (`SceneComponent.K2_GetComponentLocation` (`self.HPWidgetSocket`))))
    (:`else`
      _))
  (if (not (`self.IsPlayerDead`))
    (set `self.DistanceToPlayer` (`KismetMathLibrary.VSize` _returnvalue)) ; 플레이어와 떨어져있는 거리
    (set `self.DirectionToPlayer` (`KismetMathLibrary.Normal` _returnvalue))
    (switch `/Game/Enums/EEnemyStateType` (`self.State`)
      (:`NewEnumerator0`
        (if (<= (`self.DistanceToPlayer`) 500.0)
          (set `self.State` "NewEnumerator1")))
      (:`NewEnumerator1`
        (if (<= (`self.DistanceToPlayer`) 160.0)
          (set `self.State` "NewEnumerator2") ; approach 이후 최초 공격 상태
          (`self.PlayAnimMontage` "/Game/Mixamo/Enemy/Animations/Great_Sword_Slash_Montage.Great_Sword_Slash_Montage" (`self.AttackSpeed`))
          (set `self.isAttacking` true) ; 공격 몽타주 이후에 공격 상태 true
          (else
            (`self.AddMovementInput` (`self.DirectionToPlayer`)) ; 160미터 안에 안들어왔을 때 계속 approach
          )))
      (:`NewEnumerator2`
        (if (`self.isAttacking`)
          _
          (elif (> (`self.DistanceToPlayer`) 160.0)
            (set `self.State` "NewEnumerator1"))))
      (:`NewEnumerator3`
        (`KismetSystemLibrary.Delay` 5.0)
        (`self.K2_DestroyActor`)))))

(event `OnCollision`
  ;[1 1 1] 충돌체 켜고 끄기
  (`PrimitiveComponent.SetCollisionEnabled` (`self.SwordCollision`) "QueryAndPhysics"))

(event `OffCollision`
  ;[1 1 1] 충돌체 켜고 끄기
  (`PrimitiveComponent.SetCollisionEnabled` (`self.SwordCollision`) "NoCollision"))

(event `self.SwordCollision.OnComponentBeginOverlap`
  (params (OverlappedComponent :type "PrimitiveComponent Object Reference") (OtherActor :type "Actor Object Reference") (OtherComp :type "PrimitiveComponent Object Reference") (OtherBodyIndex :type Integer) (bFromSweep :type Boolean) (SweepResult :type "HitResult Structure (by ref)"))
  (bind _componenttags (`ActorComponent.ComponentTags` OtherComp))
  ;[1 1 1] 칼 충돌 이벤트
  (if (!= OtherActor self)
    (if (> (`KismetArrayLibrary.Array_Length` _componenttags) 0)
      (if (== (`|GetArrayItem` _componenttags) "Character")
        (bind _asbp_player (cast `/Game/Blueprints/Characters/BP_Player` OtherActor))
        (`GameplayStatics.ApplyDamage` _asbp_player (`self.Atk`) null self)))))

(fn `IsPlayerDead`
  (returns (isDead :type Boolean))
  (bind _asbp_player (cast `/Game/Blueprints/Characters/BP_Player` (`GameplayStatics.GetPlayerCharacter` 0)))
  (return (`/Game/Blueprints/Characters/BP_Player.isDead` _asbp_player)))

(fn `OnRep_CurrentHP`
  (bind _aswb_enemy_hp (cast `/Game/Widgets/WB_EnemyHP` (`WidgetComponent.GetUserWidgetObject` (`/Game/Blueprints/etc/BP_EnemyHP.Widget` (`self.EnemyHP`)))))
  (`/Game/Widgets/WB_EnemyHP.UpdateHealth` _aswb_enemy_hp (`self.CurrentHP`) (`self.MaxHP`)))

(fn `PlayDamageText`
  (bind _returnvalue (`|SpawnActorFromClass` "/Game/Blueprints/etc/BP_DamageText.BP_DamageText_C" (`KismetMathLibrary.MakeTransform` (+ (`self.K2_GetActorLocation`) (-50.0 0.0 20.0))) "Undefined" "OverrideRootScale" null null)) ; heap할당된 메모리 주소가 여기로 리턴됨
  (`/Game/Blueprints/etc/BP_DamageText.SetDamageText` _returnvalue (`self.Damage`)))

(fn `UserConstructionScript`)