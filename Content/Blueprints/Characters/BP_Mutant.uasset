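; BP_Mutant is a boss enemy that chases and attacks the player along the Y axis.
; A Tick-driven state machine handles approach, attack and death, with a timer counter choosing between punch and glowing skill swipe at randomized thresholds.
; Montage attacks pair with toggleable hit colliders that damage the player.
; Damage triggers flash, sound and floating text, CurrentHP's OnRep updates the boss HUD, and death adds slow motion and camera shake.
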(event `self.ReceiveBeginPlay`
  ;[1 1 1] BeginPlay : 다이나믹 머티리얼 생성 및 무기충돌체 끄기 등
  (bind _returnvalue (`KismetMaterialLibrary.CreateDynamicMaterialInstance` "/Game/Mixamo/Mutant/mutant_M.mutant_M"))
  (bind _output_get (set `self.DynamicMaterial` _returnvalue)) ; Material에 연결안하면 NULL
  (`PrimitiveComponent.SetMaterial` (`self.Mesh`) 0 _output_get) ; 값을 갖고있는 앞의 변수에서 값을 불러옴
  (`PrimitiveComponent.SetCollisionEnabled` (`self.PunchCollision`) "NoCollision")
  (`PrimitiveComponent.SetCollisionEnabled` (`self.SkillCollision`) "NoCollision")
  (`KismetSystemLibrary.K2_SetTimerDelegate` (delegate `IncreaseSkillTime`) 1.0 true)
  (set `self.CurrentHP` (`self.MaxHP`))
  (bind _asbp_game_instance (cast `/Game/Blueprints/Game/BP_GameInstance` (`GameplayStatics.GetGameInstance`)))
  (`/Game/Blueprints/Game/BP_GameInstance.ShowBossStatus` _asbp_game_instance false))

(event `IncreaseSkillTime`
  ;[1 1 1] BeginPlay : 다이나믹 머티리얼 생성 및 무기충돌체 끄기 등
  (`/Engine/EditorBlueprintResources/StandardMacros.IncrementFloat` (`self.SkillTime`)))

(event `DamageEffect`
  ;[1 1 1] 데미지를 입었을 때
  (`self.PlayDamageText`)
  (`MaterialInstanceDynamic.SetVectorParameterValue` (`self.DynamicMaterial`) "HitColor" (struct :`R` 1.0 :`A` 1.0))
  (`KismetSystemLibrary.Delay` 0.1)
  (`MaterialInstanceDynamic.SetVectorParameterValue` (`self.DynamicMaterial`) "HitColor" (struct :`A` 1.0)))

(event `self.ReceiveAnyDamage`
  (params (Damage :type "Float (single-precision)") (DamageType :type "DamageType Object Reference") (InstigatedBy :type "Controller Object Reference") (DamageCauser :type "Actor Object Reference"))
  ;[1 1 1] 데미지를 입었을 때
  (set `self.Damage` Damage)
  (if (`|EnumInequality` (`self.State`) "NewEnumerator3")
    (`GameplayStatics.PlaySoundAtLocation` "/Game/Sounds/Hit.Hit" (`self.K2_GetActorLocation`) (struct) 1.0 1.0 0.0 null null null)
    (`self.DamageEffect`)
    (bind _output_get (set `self.CurrentHP` (- (`self.CurrentHP`) (`self.Damage`))))
    (if (<= _output_get 0.0)
      (`GameplayStatics.SetGlobalTimeDilation` 0.25) ; 보스가 죽을 때 0.25배속
      (`PlayerCameraManager.PlayCameraShake` :`self` (`PlayerController.PlayerCameraManager` (`GameplayStatics.GetPlayerController` 0)) :`ShakeClass` "/Game/Blueprints/etc/BP_CameraShake_BossDead.BP_CameraShake_BossDead_C" :`Scale` 2.0) ; 보스가 죽을 때 카메라흔들림
      (`self.PlayAnimMontage` "/Game/Mixamo/Mutant/Animation/Mutant_Dying_Montage.Mutant_Dying_Montage" 1.0 "Start")
      (set `self.State` "NewEnumerator3")
      (`PrimitiveComponent.SetCollisionEnabled` (`self.CapsuleComponent`) "NoCollision")
      (`PrimitiveComponent.SetCollisionEnabled` (`self.PunchCollision`) "NoCollision")
      (`PrimitiveComponent.SetCollisionEnabled` (`self.SkillCollision`) "NoCollision")
      ;;[1 1 1] 보스가 죽은 후 원래 속도로 돌려줌
      (`KismetSystemLibrary.Delay` 0.2)
      (`GameplayStatics.SetGlobalTimeDilation` 1.0))))

(event `self.ReceiveTick`
  (params (DeltaSeconds :type "Float (single-precision)"))
  (bind (_returnvalue_x _returnvalue_y) (`KismetMathLibrary.BreakVector` (- (`self.K2_GetActorLocation` (`GameplayStatics.GetPlayerCharacter` 0)) (`self.K2_GetActorLocation`))))
  (bind _returnvalue (`KismetMathLibrary.MakeVector` 0.0 _returnvalue_y))
  ;[1 1 1] 상태 변경
  (if (not (`self.IsPlayerDead`))
    (set `self.DistanceToPlayer` (`KismetMathLibrary.VSize` _returnvalue)) ; 플레이어와 떨어져있는 거리
    (set `self.DirectionToPlayer` (`KismetMathLibrary.Normal` _returnvalue))
    (switch `/Game/Enums/EEnemyStateType` (`self.State`)
      (:`NewEnumerator0`
        (if (<= (`self.DistanceToPlayer`) 500.0)
          (set `self.State` "NewEnumerator1")
          (bind _asbp_game_instance (cast `/Game/Blueprints/Game/BP_GameInstance` (`GameplayStatics.GetGameInstance`)))
          (`/Game/Blueprints/Game/BP_GameInstance.ShowBossStatus` _asbp_game_instance true)))
      (:`NewEnumerator1`
        (if (<= (`self.DistanceToPlayer`) (`self.AttackRange`))
          (`self.StartAttack`)
          (else
            (`self.AddMovementInput` (`self.DirectionToPlayer`)) ; 160미터 안에 안들어왔을 때 계속 approach
          )))
      (:`NewEnumerator2`
        (if (`self.isAttacking`)
          _
          (elif (> (`self.DistanceToPlayer`) (`self.AttackRange`))
            (set `self.State` "NewEnumerator1"))))
      (:`NewEnumerator3`
        (`KismetSystemLibrary.Delay` 5.0)
        (bind _asbp_game_instance_2 (cast `/Game/Blueprints/Game/BP_GameInstance` (`GameplayStatics.GetGameInstance`)))
        (`/Game/Blueprints/Game/BP_GameInstance.ShowBossStatus` _asbp_game_instance_2 false)
        (`self.K2_DestroyActor`)))))

(event `EndAttack`
  ;[1 1 1] EndAttack : 공격종료 및 재공격
  (if (not (`self.IsPlayerDead`))
    (set `self.isAttacking` false)
    (if (> (`self.DistanceToPlayer`) (`self.AttackRange`))
      (set `self.State` "NewEnumerator1")
      (else
        (`self.StartAttack`)))))

(event `StartAttack`
  ;[1 1 1] 공격시작 -> 평타 or 스킬 분기문
  ;;[1 1 1] Mutant가 dead가 아닐 때만 공격
  ;; (죽는 몽타주 무시 방지)
  (if (not (`|EnumEquality` (`self.State`) "NewEnumerator3"))
    (`self.K2_SetActorRotation` (`KismetMathLibrary.Conv_VectorToRotator` (`self.DirectionToPlayer`)))
    (set `self.isAttacking` true) ; 공격 몽타주 이후에 공격 상태 true
    (if (>= (`self.SkillTime`) (`KismetMathLibrary.RandomFloatInRange` 2.0 5.0))
      (set `self.State` "NewEnumerator4")
      (`MaterialInstanceDynamic.SetVectorParameterValue` (`self.DynamicMaterial`) "SkillColor" (struct :`B` 20.0 :`A` 1.0))
      (`self.PlayAnimMontage` "/Game/Mixamo/Mutant/Animation/Mutant_Flexing_Muscles_Montage.Mutant_Flexing_Muscles_Montage" 3.0 "Start")
      (`KismetSystemLibrary.Delay` 0.5)
      (`MaterialInstanceDynamic.SetVectorParameterValue` (`self.DynamicMaterial`) "SkillColor" (struct :`A` 1.0))
      (if (not (<= (`self.CurrentHP`) 0.0))
        (`self.PlayAnimMontage` "/Game/Mixamo/Mutant/Animation/Mutant_Swiping_Montage.Mutant_Swiping_Montage" 2.0 "Start")
        (set `self.SkillTime` 0.0))
      (else
        (set `self.State` "NewEnumerator2")
        (`self.PlayAnimMontage` "/Game/Mixamo/Mutant/Animation/Mutant_Punch_Montage.Mutant_Punch_Montage" (`self.AttackSpeed`))))))

(event `OnCollision`
  ;[1 1 1] 충돌체 켜고 끄기
  (`PrimitiveComponent.SetCollisionEnabled` (`self.PunchCollision`) "QueryAndPhysics"))

(event `OnCollisionSkill`
  ;[1 1 1] 스킬 충돌체 켜고 / 끄기
  (`PrimitiveComponent.SetCollisionEnabled` (`self.SkillCollision`) "QueryAndPhysics"))

(event `OffCollision`
  ;[1 1 1] 충돌체 켜고 끄기
  (`PrimitiveComponent.SetCollisionEnabled` (`self.PunchCollision`) "NoCollision"))

(event `OffCollisionSkill`
  ;[1 1 1] 스킬 충돌체 켜고 / 끄기
  (`PrimitiveComponent.SetCollisionEnabled` (`self.SkillCollision`) "NoCollision"))

(event `self.PunchCollision.OnComponentBeginOverlap`
  (params (OverlappedComponent :type "PrimitiveComponent Object Reference") (OtherActor :type "Actor Object Reference") (OtherComp :type "PrimitiveComponent Object Reference") (OtherBodyIndex :type Integer) (bFromSweep :type Boolean) (SweepResult :type "HitResult Structure (by ref)"))
  (bind _componenttags (`ActorComponent.ComponentTags` OtherComp))
  ;[1 1 1] 펀치 충돌 이벤트
  (if (!= OtherActor self)
    (if (> (`KismetArrayLibrary.Array_Length` _componenttags) 0)
      (if (== (`|GetArrayItem` _componenttags) "Character")
        (bind _asbp_player (cast `/Game/Blueprints/Characters/BP_Player` OtherActor))
        (`GameplayStatics.ApplyDamage` _asbp_player (`self.Atk`) null self)))))

(event `self.SkillCollision.OnComponentBeginOverlap`
  (params (OverlappedComponent :type "PrimitiveComponent Object Reference") (OtherActor :type "Actor Object Reference") (OtherComp :type "PrimitiveComponent Object Reference") (OtherBodyIndex :type Integer) (bFromSweep :type Boolean) (SweepResult :type "HitResult Structure (by ref)"))
  (bind _componenttags (`ActorComponent.ComponentTags` OtherComp))
  ;[1 1 1] 스킬 충돌 이벤트
  (if (!= OtherActor self)
    (if (> (`KismetArrayLibrary.Array_Length` _componenttags) 0)
      (if (== (`|GetArrayItem` _componenttags) "Character")
        (bind _asbp_player (cast `/Game/Blueprints/Characters/BP_Player` OtherActor))
        (`GameplayStatics.ApplyDamage` _asbp_player (`self.SkillAtk`) null self)))))

(fn `IsPlayerDead`
  (returns (isDead :type Boolean))
  (bind _asbp_player (cast `/Game/Blueprints/Characters/BP_Player` (`GameplayStatics.GetPlayerCharacter` 0)))
  (return (`/Game/Blueprints/Characters/BP_Player.isDead` _asbp_player)))

(fn `OnRep_CurrentHP`
  (bind _asbp_game_instance (cast `/Game/Blueprints/Game/BP_GameInstance` (`GameplayStatics.GetGameInstance`)))
  (`/Game/Widgets/WB_HUD.UpdateHealth_Boss` (`/Game/Blueprints/Game/BP_GameInstance.HUDWidget` _asbp_game_instance) (`self.CurrentHP`) (`self.MaxHP`)))

(fn `PlayDamageText`
  (bind _returnvalue (`|SpawnActorFromClass` "/Game/Blueprints/etc/BP_DamageText.BP_DamageText_C" (`KismetMathLibrary.MakeTransform` (+ (`self.K2_GetActorLocation`) (-50.0 0.0 20.0))) "Undefined" "OverrideRootScale" null null))
  (`/Game/Blueprints/etc/BP_DamageText.SetDamageText` _returnvalue (`self.Damage`)))

(fn `UserConstructionScript`)