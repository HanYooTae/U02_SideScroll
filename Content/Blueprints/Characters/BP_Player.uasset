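; Side-scrolling Paladin player character with single-axis movement, jumping, a timeline-driven roll and a three-hit sword combo.
; Montage attacks use toggled sword collision, with an AddUnique array preventing repeat hits per swing, plus a shield overlap damage handler.
; Damage triggers floating text, a material flash and death at zero HP, while CurrentHP's RepNotify updates the HUD.
; It also handles potion pickups, pausing and cheat/debug keys for kill-all, slow motion and ragdoll.
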(event `Key|X`
  (params (Key :type "Key Structure"))
  ;[1 0.2562 0.9129] 치트키
  (:`Pressed`
    (bind _asbp_game_mode (cast `/Game/Blueprints/Game/BP_GameMode` (`GameplayStatics.GetGameMode`)))
    (`/Game/Blueprints/Game/BP_GameMode.KillAllMutant` _asbp_game_mode)))

(event `Key|C`
  (params (Key :type "Key Structure"))
  ;[1 1 1] 슬로우
  (:`Pressed`
    (`GameplayStatics.SetGlobalTimeDilation` 0.25))
  (:`Released`
    (`GameplayStatics.SetGlobalTimeDilation` 1.0)))

(event `Key|Q`
  (params (Key :type "Key Structure"))
  (:`Pressed`
    (`PrimitiveComponent.SetSimulatePhysics` (`self.Mesh`) true)
    (`PrimitiveComponent.SetCollisionEnabled` (`self.Mesh`) "QueryAndPhysics")
    (`PrimitiveComponent.SetCollisionEnabled` (`self.CapsuleComponent`) "NoCollision")))

(event `self.ReceiveBeginPlay`
  ;[1 1 1] BeginPlay -> 카메라 세팅
  (`PlayerController.SetViewTargetWithBlend` (`GameplayStatics.GetPlayerController` 0) (`self.Camera`) 0.0 "VTBlend_Linear" 0.0 false)
  (`PrimitiveComponent.SetCollisionEnabled` (`self.SwordCollision`) "NoCollision")
  (`PrimitiveComponent.SetCollisionEnabled` (`self.ShieldCollision`) "NoCollision")
  (bind _returnvalue (`KismetMaterialLibrary.CreateDynamicMaterialInstance` "/Game/Mixamo/Paladin/Paladin_MAT_Inst.Paladin_MAT_Inst"))
  (bind _output_get (set `self.DynamicMaterial` _returnvalue))
  (`PrimitiveComponent.SetMaterial` (`self.Mesh`) 0 _output_get)
  (bind _asbp_game_instance (cast `/Game/Blueprints/Game/BP_GameInstance` (`GameplayStatics.GetGameInstance`)))
  (`/Game/Blueprints/Game/BP_GameInstance.ShowPlayerStatus` _asbp_game_instance true)
  (set `self.CurrentHP` (`self.MaxHP`)))

(event `InputAxis|MoveRight`
  (params (AxisValue :type "Float (single-precision)"))
  ;[1 1 1] 이동
  (`self.UpdateLastAxis` AxisValue)
  (if (`self.IsAttacking`)
    _
    (elif (not (`self.isRolling`))
      (`self.AddMovementInput` (0.0 1.0 0.0) AxisValue))))

(event `Key|SpaceBar`
  (params (Key :type "Key Structure"))
  ;[1 1 1] 점프
  (:`Pressed`
    (if (`self.IsAttacking`)
      _
      (elif (not (`self.isRolling`))
        (`self.Jump`)
        (`GameplayStatics.PlaySoundAtLocation` "/Game/Sounds/Jump.Jump" (`self.K2_GetActorLocation`) (struct) 1.0 1.0 0.0 null null null))))
  (:`Released`
    (`self.StopJumping`)))

(event `Key|LeftShift`
  (params (Key :type "Key Structure"))
  (bind _returnvalue (`self.K2_GetActorLocation`))
  ;[1 1 1] 구르기
  (:`Pressed`
    (if (not (`self.isRolling`))
      (set `self.isRolling` true)
      (`self.EndAttack`)
      (`self.OffCollision`)
      (`self.ForceRotationByAxis`)
      (`self.PlayAnimMontage` "/Game/Mixamo/Paladin/Animations/Sprinting_Forward_Roll_Montage.Sprinting_Forward_Roll_Montage" 1.5)
      (`TimelineComponent.SetPlayRate` (`self.RollTimeline`) 1.8)
      (bind (_direction _output) (`Timeline|RollTimeline` :!via `PlayFromStart`)
        (:`Update`
          (`self.K2_SetActorLocation` (`KismetMathLibrary.VLerp` _returnvalue (+ _returnvalue (* (`self.GetActorForwardVector`) 10.0)) _output) true))))))

(event `BeginSpectator`
  ;[1 1 1] 구르기
  (`PrimitiveComponent.SetCollisionProfileName` (`self.CapsuleComponent`) "Spectator" true))

(event `EndSpectator`
  ;[1 1 1] 구르기
  (`PrimitiveComponent.SetCollisionProfileName` (`self.CapsuleComponent`) "Pawn" true))

(event `Key|LeftMouseButton`
  (params (Key :type "Key Structure"))
  ;[1 1 1] 공격
  (:`Pressed`
    (if (`self.isRolling`)
      _
      (elif (`self.IsAttacking`)
        (set `self.isNextCombo` true)
        (else
          (set `self.IsAttacking` true)
          (`self.ForceRotationByAxis`)
          (`self.PlayAnimMontage` "/Game/Mixamo/Paladin/Animations/sword_and_shield_slash_Montage.sword_and_shield_slash_Montage" 1.5))))))

(event `NextCombo`
  ;[1 1 1] 공격
  (if (`self.isNextCombo`)
    (set `self.isNextCombo` false)
    (bind _result (`/Engine/EditorBlueprintResources/StandardMacros.IncrementInt` (`self.ComboCount`))
      (:`  `
        (switch `int` _result
          (:`1`
            (`self.PlayAnimMontage` "/Game/Mixamo/Paladin/Animations/Standing_Melee_Attack_Backhand_Montage.Standing_Melee_Attack_Backhand_Montage" 1.75))
          (:`2`
            (`self.PlayAnimMontage` "/Game/Mixamo/Paladin/Animations/Standing_Melee_Attack_360_High_Montage.Standing_Melee_Attack_360_High_Montage" 2.0)))))))

(event `EndRolling`
  ;[1 1 1] 구르기
  (set `self.isRolling` false))

(event `EndAttack`
  ;[1 1 1] 공격
  (set `self.IsAttacking` false)
  (set `self.ComboCount` 0))

(event `self.SwordCollision.OnComponentBeginOverlap`
  (params (OverlappedComponent :type "PrimitiveComponent Object Reference") (OtherActor :type "Actor Object Reference") (OtherComp :type "PrimitiveComponent Object Reference") (OtherBodyIndex :type Integer) (bFromSweep :type Boolean) (SweepResult :type "HitResult Structure (by ref)"))
  (bind _componenttags (`ActorComponent.ComponentTags` OtherComp))
  (bind _output (`|GetArrayItem` _componenttags))
  ;[1 1 1] 칼 충돌 이벤트
  (set `self.OtherActor` OtherActor)
  (set `self.SweepResult` SweepResult)
  (if (!= (`self.OtherActor`) self)
    (if (> (`KismetArrayLibrary.Array_Length` _componenttags) 0)
      (if (or (== _output "Character") (== _output "itemBox"))
        (if (`self.isNotMultiHitted`)
          (`GameplayStatics.ApplyPointDamage` (`self.OtherActor`) (`|GetArrayItem` (`self.Atk`) (`self.ComboCount`)) (`self.K2_GetActorLocation` (`self.OtherActor`)) (`self.SweepResult`) null self)
          (`PlayerController.ClientStartCameraShake` :`self` (`GameplayStatics.GetPlayerController` 0) :`Shake` "/Game/Blueprints/etc/BP_CameraShake_Hit.BP_CameraShake_Hit_C")
          (`GameplayStatics.SpawnEmitterAtLocation` "/Game/InfinityBladeEffects/Effects/FX_Mobile/Fire/combat/P_FireBall_Powerup.P_FireBall_Powerup" (`SceneComponent.K2_GetComponentLocation` (`self.SwordCollision`))))))))

(event `self.ShieldCollision.OnComponentBeginOverlap`
  (params (OverlappedComponent :type "PrimitiveComponent Object Reference") (OtherActor :type "Actor Object Reference") (OtherComp :type "PrimitiveComponent Object Reference") (OtherBodyIndex :type Integer) (bFromSweep :type Boolean) (SweepResult :type "HitResult Structure (by ref)"))
  (bind _componenttags (`ActorComponent.ComponentTags` OtherComp))
  (bind _output (`|GetArrayItem` _componenttags))
  ;[1 1 1] 방패 충돌 이벤트
  (if (!= OtherActor self)
    (if (> (`KismetArrayLibrary.Array_Length` _componenttags) 0)
      (if (or (== _output "Character") (== _output "itemBox"))
        (`GameplayStatics.ApplyDamage` OtherActor (`|GetArrayItem` (`self.Atk`) (`self.ComboCount`)) null self) ; Damaged Actor에게 데미지를 준다
        (`PlayerController.ClientStartCameraShake` :`self` (`GameplayStatics.GetPlayerController` 0) :`Shake` "/Game/Blueprints/etc/BP_CameraShake_Hit.BP_CameraShake_Hit_C")
        (`GameplayStatics.SpawnEmitterAtLocation` null (`SceneComponent.K2_GetComponentLocation` (`self.ShieldCollision`)))))))

(event `OnCollision`
  ;[1 1 1] 충돌체 켜고 끄기
  (`PrimitiveComponent.SetCollisionEnabled` (`self.SwordCollision`) "QueryAndPhysics"))

(event `OffCollision`
  ;[1 1 1] 충돌체 켜고 끄기
  (`PrimitiveComponent.SetCollisionEnabled` (`self.SwordCollision`) "NoCollision")
  ;[1 1 1] 다단히트 감시 배열 초기화(isNotMultiHitted)
  (`KismetArrayLibrary.Array_Clear` (`self.HittedActors`)))

(event `self.ReceiveAnyDamage`
  (params (Damage :type "Float (single-precision)") (DamageType :type "DamageType Object Reference") (InstigatedBy :type "Controller Object Reference") (DamageCauser :type "Actor Object Reference"))
  ;[1 1 1] 데미지를 입었을 때
  (if (not (`self.isDead`))
    (set `self.Damage` Damage)
    (`GameplayStatics.PlaySoundAtLocation` "/Game/Sounds/PaladinHit.PaladinHit" (`self.K2_GetActorLocation`) (struct) 1.0 1.0 0.0 null null null)
    (`self.DamageEffect`)
    (set `self.CurrentHP` (- (`self.CurrentHP`) (`self.Damage`)))
    (if (<= (`self.CurrentHP`) 0.0)
      (`self.PlayAnimMontage` "/Game/Mixamo/Paladin/Animations/sword_and_shield_death__2__Montage.sword_and_shield_death__2__Montage")
      (set `self.isDead` true)
      (`self.DisableInput` null) ; 죽었을 때 키입력 중단
      (`PrimitiveComponent.SetCollisionEnabled` (`self.Mesh`) "NoCollision"))))

(event `DamageEffect`
  ;[1 1 1] 데미지를 입었을 때
  (`self.PlayDamageText`)
  (`MaterialInstanceDynamic.SetVectorParameterValue` (`self.DynamicMaterial`) "HitColor" (struct :`R` 1.0 :`A` 1.0))
  (`KismetSystemLibrary.Delay` 0.1)
  (`MaterialInstanceDynamic.SetVectorParameterValue` (`self.DynamicMaterial`) "HitColor" (struct :`A` 1.0)))

(event `Key|Escape`
  (params (Key :type "Key Structure"))
  (bind _returnvalue (`GameplayStatics.GetGameMode`))
  (bind _returnvalue_2 (`GameplayStatics.GetPlayerController` 0))
  (bind _returnvalue_3 (`GameplayStatics.GetPlayerController` 0))
  ;[1 1 1] 일지중지(delta time = 0)
  (:`Pressed`
    (`GameplayStatics.SetGamePaused` true :!label _label)
    ;[1 1 1] 일시중지 UI
    (bind _asbp_game_mode (cast `/Game/Blueprints/Game/BP_GameMode` _returnvalue)
      (:`then`
        (`Widget.SetVisibility` (`/Game/Blueprints/Game/BP_GameMode.PauseWidget` _asbp_game_mode) "Visible")
        (set `PlayerController.bShowMouseCursor` true _returnvalue_3)
        (`WidgetBlueprintLibrary.SetInputMode_UIOnlyEx` _returnvalue_3 null))
      (:`CastFailed`
        (bind _asbp_game_mode_final_stage (cast `/Game/Blueprints/Game/BP_GameMode_FinalStage` _returnvalue))
        (`Widget.SetVisibility` (`/Game/Blueprints/Game/BP_GameMode_FinalStage.PauseWidget` _asbp_game_mode_final_stage) "Visible")
        (set `PlayerController.bShowMouseCursor` true _returnvalue_2)
        (`WidgetBlueprintLibrary.SetInputMode_UIOnlyEx` _returnvalue_2 null)))))

(event `Key|F10`
  (params (Key :type "Key Structure"))
  ;[1 1 1] 일지중지(delta time = 0)
  (:`Pressed`
    (goto _label)))

(event `self.CapsuleComponent.OnComponentBeginOverlap`
  (params (OverlappedComponent :type "PrimitiveComponent Object Reference") (OtherActor :type "Actor Object Reference") (OtherComp :type "PrimitiveComponent Object Reference") (OtherBodyIndex :type Integer) (bFromSweep :type Boolean) (SweepResult :type "HitResult Structure (by ref)"))
  ;[1 1 1] 포션 먹기
  (bind _asbp_potion (cast `/Game/Blueprints/etc/BP_Potion` OtherActor))
  (`/Game/Blueprints/etc/BP_Potion.IncreaseHP` _asbp_potion self)
  (`GameplayStatics.PlaySound2D` "/Game/Sounds/FairyDrop.FairyDrop" 1.0 1.0 0.0 null null)
  (`GameplayStatics.SpawnEmitterAttached` "/Game/InfinityBladeEffects/Effects/FX_Ability/Heal/P_Health_Pickup_01.P_Health_Pickup_01" (`self.CapsuleComponent`) "None" (0.0 0.0 0.0) (struct) (1.0 1.5 1.0))
  (`self.K2_DestroyActor` _asbp_potion))

(fn `ForceRotationByAxis`
  (if (`self.isRight`)
    (`self.K2_SetActorRotation` (struct :`Yaw` 90.0))
    (else
      (`self.K2_SetActorRotation` (struct :`Yaw` -90.0)))))

(fn `isNotMultiHitted`
  (returns (ReturnValue :type Boolean))
  (locals (`이전에 충돌됐던 충돌체의 갯수` :type Integer))
  (set `local.이전에 충돌됐던 충돌체의 갯수` (`KismetArrayLibrary.Array_Length` (`self.HittedActors`)))
  (`KismetArrayLibrary.Array_AddUnique` (`self.HittedActors`) (`self.OtherActor`)) ; 이미 추가된 주소는 배열에 또 추가하지 않음
  (return (< (`local.이전에 충돌됐던 충돌체의 갯수`) (`KismetArrayLibrary.Array_Length` (`self.HittedActors`)))))

(fn `OnRep_CurrentHP`
  (bind _asbp_game_instance (cast `/Game/Blueprints/Game/BP_GameInstance` (`GameplayStatics.GetGameInstance`)))
  (`/Game/Widgets/WB_HUD.UpdateHealth` (`/Game/Blueprints/Game/BP_GameInstance.HUDWidget` _asbp_game_instance) (`self.CurrentHP`) (`self.MaxHP`)))

(fn `PlayDamageText`
  (bind _returnvalue (`|SpawnActorFromClass` "/Game/Blueprints/etc/BP_DamageText.BP_DamageText_C" (`KismetMathLibrary.MakeTransform` (+ (`self.K2_GetActorLocation`) (-50.0 0.0 20.0))) "Undefined" "OverrideRootScale" null null))
  (`/Game/Blueprints/etc/BP_DamageText.SetDamageText` _returnvalue (`self.Damage`)))

(fn `UpdateLastAxis`
  (params (AxisValue :type "Float (double-precision)"))
  (if (< AxisValue 0.0)
    (set `self.isRight` false)
    (elif (> (`local.AxisValue`) 0.0)
      (set `self.isRight` true))))

(fn `UserConstructionScript`)