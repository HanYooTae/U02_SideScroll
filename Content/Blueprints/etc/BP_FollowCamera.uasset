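; BP_FollowCamera is a camera actor that smoothly follows the first player character at a fixed offset.
; BeginPlay records the offset between the camera and the character, preserving their initial placement.
; Each Tick lerps the camera's location toward the character position plus that offset, using DeltaSeconds times FollowSpeed as alpha for a lagging follow.
; Only location changes; rotation is never touched.
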(event `self.ReceiveBeginPlay`
  (set `self.Offset` (- (`self.K2_GetActorLocation`) (`self.K2_GetActorLocation` (`GameplayStatics.GetPlayerCharacter` 0)))) ; 카메라와 캐릭터가 떨어진 간격
)

(event `self.ReceiveTick`
  (params (DeltaSeconds :type "Float (single-precision)"))
  (`self.K2_SetActorLocation` (`KismetMathLibrary.VLerp` (`self.K2_GetActorLocation`) (+ (`self.K2_GetActorLocation` (`GameplayStatics.GetPlayerCharacter` 0)) (`self.Offset`)) (* DeltaSeconds (`self.FollowSpeed`)))))

(fn `UserConstructionScript`)