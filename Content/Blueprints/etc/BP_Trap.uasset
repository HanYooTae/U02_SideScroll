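; BP_Trap is a spinning trap actor that deals repeated damage to any Character overlapping it.
; Begin and end overlap events maintain the OtherCharacters list, starting a short looping timer on entry and clearing it once the list is empty.
; Each timer call to TakeTrapDamage applies ATK damage to every listed character.
; Tick rotates the actor by a fixed step per frame, so spin speed depends on frame rate.
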(event `self.ReceiveActorBeginOverlap`
  (params (OtherActor :type "Actor Object Reference"))
  (bind _ascharacter (cast `Character` OtherActor))
  (`KismetArrayLibrary.Array_AddUnique` (`self.OtherCharacters`) _ascharacter)
  (bind _returnvalue (`KismetSystemLibrary.K2_SetTimer` self "TakeTrapDamage" 0.1 true))
  (set `self.TimerHandle` _returnvalue))

(event `self.ReceiveActorEndOverlap`
  (params (OtherActor :type "Actor Object Reference"))
  (bind _ascharacter (cast `Character` OtherActor))
  (`KismetArrayLibrary.Array_RemoveItem` (`self.OtherCharacters`) _ascharacter)
  (if (< (`KismetArrayLibrary.Array_Length` (`self.OtherCharacters`)) 1)
    (`KismetSystemLibrary.K2_ClearAndInvalidateTimerHandle` (`self.TimerHandle`))))

(event `self.ReceiveTick`
  (params (DeltaSeconds :type "Float (single-precision)"))
  (`self.K2_AddActorWorldRotation` (struct :`Roll` 5.0)))

(fn `TakeTrapDamage`
  (for _array_element (`self.OtherCharacters`)
    (`GameplayStatics.ApplyDamage` _array_element (`self.ATK`) null self)))

(fn `UserConstructionScript`)