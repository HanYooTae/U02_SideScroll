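; A trigger actor that plays the Master_BossEncounter level sequence once, when the player first overlaps it.
; During playback it reveals its initially hidden CinematicActors, hides the player status UI, disables player input, and hides and stops ticking on every Character and BP_EnemyHP actor.
; A timer set to the sequence's end time restores gameplay actors, input and UI, then destroys the cinematic actors.
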(event `OnFinishCinematics`
  (bind _outactors (`GameplayStatics.GetAllActorsOfClass` "/Script/Engine.Actor"))
  (for _array_element _outactors
    (bind _returnvalue (`GameplayStatics.GetObjectClass` _array_element))
    (if (or (`KismetMathLibrary.ClassIsChildOf` _returnvalue "/Script/Engine.Character") (`KismetMathLibrary.ClassIsChildOf` _returnvalue "/Game/Blueprints/etc/BP_EnemyHP.BP_EnemyHP_C"))
      (`self.SetActorHiddenInGame` _array_element false)
      (`self.SetActorTickEnabled` _array_element true)))
  (`self.EnableInput` (`GameplayStatics.GetPlayerCharacter` 0) (`GameplayStatics.GetPlayerController` 0))
  (bind _asbp_game_instance (cast `/Game/Blueprints/Game/BP_GameInstance` (`GameplayStatics.GetGameInstance`)))
  (`/Game/Blueprints/Game/BP_GameInstance.ShowPlayerStatus` _asbp_game_instance true)
  (for _array_element_2 (`self.CinematicActors`)
    (`self.K2_DestroyActor` _array_element_2)))

(event `self.ReceiveBeginPlay`
  (for _array_element (`self.CinematicActors`)
    (`self.SetActorHiddenInGame` _array_element true)))

(event `self.ReceiveActorBeginOverlap`
  (params (OtherActor :type "Actor Object Reference"))
  (cast `/Game/Blueprints/Characters/BP_Player` OtherActor)
  (`/Engine/EditorBlueprintResources/StandardMacros.DoOnce` false
    (:`Completed`
      (for _array_element (`self.CinematicActors`)
        (`self.SetActorHiddenInGame` _array_element false))
      (bind _asbp_game_instance (cast `/Game/Blueprints/Game/BP_GameInstance` (`GameplayStatics.GetGameInstance`)))
      (`/Game/Blueprints/Game/BP_GameInstance.ShowPlayerStatus` _asbp_game_instance false)
      (bind (_outactor _returnvalue) (`LevelSequencePlayer.CreateLevelSequencePlayer` "/Game/Cinematics/Master_BossEncounter.Master_BossEncounter"))
      (`KismetSystemLibrary.K2_SetTimerDelegate` (delegate `OnFinishCinematics`) (`TimeManagementBlueprintLibrary.Conv_QualifiedFrameTimeToSeconds` (`MovieSceneSequencePlayer.GetEndTime` _returnvalue)))
      (`self.DisableInput` (`GameplayStatics.GetPlayerCharacter` 0) (`GameplayStatics.GetPlayerController` 0))
      (`MovieSceneSequencePlayer.Play` _returnvalue) ; Level Sequence 재생
      (bind _outactors (`GameplayStatics.GetAllActorsOfClass` "/Script/Engine.Actor"))
      (for _array_element_2 _outactors
        (bind _returnvalue_2 (`GameplayStatics.GetObjectClass` _array_element_2))
        (if (or (`KismetMathLibrary.ClassIsChildOf` _returnvalue_2 "/Script/Engine.Character") (`KismetMathLibrary.ClassIsChildOf` _returnvalue_2 "/Game/Blueprints/etc/BP_EnemyHP.BP_EnemyHP_C"))
          (`self.SetActorHiddenInGame` _array_element_2 true)
          (`self.SetActorTickEnabled` _array_element_2 false))))))

(fn `UserConstructionScript`)