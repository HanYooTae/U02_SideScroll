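; BP_DamageText is a floating damage number actor that animates on spawn and then removes itself.
; SetDamageText writes the damage value to its TextRender component.
; On BeginPlay, a Timeline drives the text from its start location, using the X output as a world Z offset and the Y output as a uniform scale.
; The actor destroys itself when the Timeline finishes.
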(event `self.ReceiveBeginPlay`
  (set `self.StartLocation` (`self.K2_GetActorLocation`))
  (bind (_direction _output) (`Timeline|Timeline`)
    (:`Update`
      (`SceneComponent.K2_SetWorldLocation` (`self.TextRender`) (+ (`self.StartLocation`) (`KismetMathLibrary.MakeVector` 0.0 0.0 (.x _output))) false false) ; text Z축의 위치 변경
      (`SceneComponent.SetWorldScale3D` (`self.TextRender`) (`KismetMathLibrary.Conv_DoubleToVector` (.y _output))) ; text 크기 변경
    )
    (:`Finished`
      (`self.K2_DestroyActor`))))

(fn `SetDamageText`
  (params (Damage :type "Float (double-precision)"))
  (`TextRenderComponent.K2_SetText` (`self.TextRender`) (`KismetTextLibrary.Conv_DoubleToText` Damage "HalfToEven")))

(fn `UserConstructionScript`)