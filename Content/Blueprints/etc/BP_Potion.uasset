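; BP_Potion is a health potion actor that floats up and down and can restore a player's HP.
; On BeginPlay it sets a target a short distance along its up vector, then a slowed Timeline lerps its location toward it.
; The Timeline's Finished output re-enters a FlipFlop that alternates Play and Reverse, looping the bob.
; IncreaseHP adds Amount to the given player's CurrentHP, clamped to MaxHP; nothing here calls it.
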(event `self.ReceiveBeginPlay`
  (bind _output_get (set `self.StartLocation` (`self.K2_GetActorLocation`)))
  (set `self.TargetLocation` (+ _output_get (* (`self.GetActorUpVector`) 50.0)))
  (`TimelineComponent.SetPlayRate` (`self.Timeline`) 0.25)
  (`/Engine/EditorBlueprintResources/StandardMacros.FlipFlop` :!label _label
    (:`A`
      (bind (_direction _output) (`Timeline|Timeline` :!label _label_2)
        (:`Update`
          (`self.K2_SetActorLocation` (`KismetMathLibrary.VLerp` (`self.StartLocation`) (`self.TargetLocation`) _output)))
        (:`Finished`
          (goto _label))))
    (:`B`
      (goto _label_2 :!via `Reverse`))))

(fn `IncreaseHP`
  (params (isPlayer :type "/Game/Blueprints/Characters/BP_Player Object Reference"))
  (bind _isplayer (`local.isPlayer`))
  (set `/Game/Blueprints/Characters/BP_Player.CurrentHP` (`KismetMathLibrary.FClamp` (+ (`/Game/Blueprints/Characters/BP_Player.CurrentHP` isPlayer) (`self.Amount`)) 0.0 (`/Game/Blueprints/Characters/BP_Player.MaxHP` _isplayer)) _isplayer))

(fn `UserConstructionScript`)